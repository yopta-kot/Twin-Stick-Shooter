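; BP_Door is a sliding door that opens and closes through the Open/CloseDoor event while a BP_TSSBaseCharacter is nearby.
; Box overlaps set the CharacterNearDoor flag and show or hide the Hit component.
; Each valid toggle calls OnOffTeleportMessage on TeleportRef, and a FlipFlop plays or reverses a Timeline that slides Cube along relative X.
; A dynamic material color snippet is left unconnected.
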(event `/Game/Blueprints/Door/BPI_Door.Open/Close Door`
  ;[1 1 1] Check CharacterNearDoor
  (if (`self.CharacterNearDoor`)
    (message `/Game/Blueprints/Teleport/BPI_TeleportActivation.On/Off Teleport` (`self.TeleportRef`))
    ;[1 1 1] Open/Close door
    (`/Engine/EditorBlueprintResources/StandardMacros.FlipFlop`
      (:`A`
        (bind (_direction _angle) (`Timeline|Timeline` :!via `PlayFromStart` :!label _label)
          (:`Update`
            (`SceneComponent.K2_SetRelativeLocation` (`self.Cube`) (`KismetMathLibrary.MakeVector` (`KismetMathLibrary.Lerp` 0.0 100.0 _angle)) false false))))
      (:`B`
        (goto _label :!via `Reverse`)))))

(event `self.Box.OnComponentBeginOverlap`
  (params (OverlappedComponent :type "PrimitiveComponent Object Reference") (OtherActor :type "Actor Object Reference") (OtherComp :type "PrimitiveComponent Object Reference") (OtherBodyIndex :type Integer) (bFromSweep :type Boolean) (SweepResult :type "HitResult Structure (by ref)"))
  ;[1 1 1] Begin Overlap and setting CharacterNearDoor as True if cast do successfully
  (cast `/Game/Player/BP_TSSBaseCharacter` OtherActor)
  (set `self.CharacterNearDoor` true)
  (`SceneComponent.SetVisibility` (`self.Hit`) true false))

(event `self.Box.OnComponentEndOverlap`
  (params (OverlappedComponent :type "PrimitiveComponent Object Reference") (OtherActor :type "Actor Object Reference") (OtherComp :type "PrimitiveComponent Object Reference") (OtherBodyIndex :type Integer))
  ;[1 1 1] End Overlap and setting CharacterNearDoor as False if cast do successfully
  (cast `/Game/Player/BP_TSSBaseCharacter` OtherActor)
  (set `self.CharacterNearDoor` false)
  (`SceneComponent.SetVisibility` (`self.Hit`) false false))

(fn `UserConstructionScript`)