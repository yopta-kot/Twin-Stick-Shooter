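; Blockout sliding door that toggles open and closed on an Open/CloseDoor event while a TSS base character stands in its trigger box.
; The toggle also calls the on/off message on a teleport reference, then a FlipFlop plays or reverses a timeline that slides the cube along X by an offset, with sound.
; Leaving the box can auto-close an open door through the same FlipFlop, if that option is enabled.
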(event `self.Open/Close Door`
  ;[1 1 1] Check CharacterNearDoor
  (if (`self.CharacterNearDoor`)
    (message `/Game/Blueprints/Teleport/BPI_TeleportActivation.On/Off Teleport` (`self.TeleportRef`))
    ;[1 1 1] Open/Close door
    (`/Engine/EditorBlueprintResources/StandardMacros.FlipFlop` :!label _label
      (:`A`
        (set `self.IsDoorOpened?` true)
        (`GameplayStatics.PlaySound2D` "/Game/Blueprints/Door/SFX/SFX_OpenCloseDoor.SFX_OpenCloseDoor" 1.0 1.0 0.0 null null)
        (bind (_direction _angle) (`Timeline|Timeline` :!via `PlayFromStart` :!label _label_2)
          (:`Update`
            (`SceneComponent.K2_SetRelativeLocation` (`self.Cube`) (`KismetMathLibrary.MakeVector` (`KismetMathLibrary.Lerp` 0.0 (`self.Offset`) _angle)) false false))))
      (:`B`
        (set `self.IsDoorOpened?` false)
        (`GameplayStatics.PlaySound2D` "/Game/Blueprints/Door/SFX/SFX_OpenCloseDoor.SFX_OpenCloseDoor" 1.0 1.0 0.0 null null)
        (goto _label_2 :!via `Reverse`)))))

(event `CloseDoor`
  (goto _label))

(event `self.Box.OnComponentBeginOverlap`
  (params (OverlappedComponent :type "PrimitiveComponent Object Reference") (OtherActor :type "Actor Object Reference") (OtherComp :type "PrimitiveComponent Object Reference") (OtherBodyIndex :type Integer) (bFromSweep :type Boolean) (SweepResult :type "HitResult Structure (by ref)"))
  ;[1 1 1] Begin Overlap and setting CharacterNearDoor as True if cast do successfully
  (cast `/Game/Player/BP_TSSBaseCharacter` OtherActor)
  (set `self.CharacterNearDoor` true))

(event `self.Box.OnComponentEndOverlap`
  (params (OverlappedComponent :type "PrimitiveComponent Object Reference") (OtherActor :type "Actor Object Reference") (OtherComp :type "PrimitiveComponent Object Reference") (OtherBodyIndex :type Integer))
  ;[1 1 1] End Overlap and setting CharacterNearDoor as False if cast do successfully
  (cast `/Game/Player/BP_TSSBaseCharacter` OtherActor)
  (set `self.CharacterNearDoor` false)
  (if (and (`self.IsCloseAfterEndOverlaped`) (`self.IsDoorOpened?`))
    (`self.CloseDoor`)))

(fn `UserConstructionScript`)