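; Blockout teleporter that moves a character entering its box to the TeleportEnd actor's location and resets level pickups.
; A DoOnce gates the box overlap and continues only for BP_TSSBaseCharacter actors.
; Before moving the character, it respawns every static, picked-up BP_Ammo and BP_Health in the world.
; A three-minute delay then calls Restart, which resets the DoOnce to re-arm the teleporter.
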(event `Restart`
  (goto _label :!via `Reset`))

(event `self.Box.OnComponentBeginOverlap`
  (params (OverlappedComponent :type "PrimitiveComponent Object Reference") (OtherActor :type "Actor Object Reference") (OtherComp :type "PrimitiveComponent Object Reference") (OtherBodyIndex :type Integer) (bFromSweep :type Boolean) (SweepResult :type "HitResult Structure (by ref)"))
  (`/Engine/EditorBlueprintResources/StandardMacros.DoOnce` false :!label _label
    (:`Completed`
      (bind _asbp_tssbase_character (cast `/Game/Player/BP_TSSBaseCharacter` OtherActor))
      (`|ExecutionSequence`
        (:`then_0`
          (bind _outactors (`GameplayStatics.GetAllActorsOfClass` "/Game/Pickups/BP_Ammo.BP_Ammo_C"))
          (for _array_element _outactors
            (if (and (`/Game/Pickups/BP_Ammo.IsStatic?` _array_element) (`/Game/Pickups/BP_Ammo.IsPickuped?` _array_element))
              (`/Game/Pickups/BP_Ammo.Respawn` _array_element))))
        (:`then_1`
          (bind _outactors_2 (`GameplayStatics.GetAllActorsOfClass` "/Game/Pickups/BP_Health.BP_Health_C"))
          (for _array_element_2 _outactors_2
            (if (and (`/Game/Pickups/BP_Health.IsStatic?` _array_element_2) (`/Game/Pickups/BP_Health.IsPickuped?` _array_element_2))
              (`/Game/Pickups/BP_Health.Respawn` _array_element_2))))
        (:`then_2`
          (`self.K2_SetActorLocation` _asbp_tssbase_character (`self.K2_GetActorLocation` (`self.TeleportEnd`)) false false)
          (`KismetSystemLibrary.Delay` (* 3.0 60.0))
          (`self.Restart`))))))

(fn `UserConstructionScript`)