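; Base enemy character that takes projectile damage and shows its health as floating text kept at a fixed pitch.
; On BeginPlay it spawns a damage hitbox actor attached to a mesh socket.
; Capsule overlaps with BP_TSSProjectile reduce health.
; Death stops AI logic, awards score through the game mode, notifies the enemy spawner, randomly drops a weighted pickup and destroys the actor after a delay.
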(event `self.ReceiveBeginPlay`
  (`self.SetHealthText`)
  (bind _returnvalue (`|SpawnActorFromClass` "/Game/Enemy/BP_EnemyHitBox.BP_EnemyHitBox_C" (`self.GetTransform`) "Undefined" "MultiplyWithRoot" self self))
  (bind _output_get (set `self.HitBoxRef` _returnvalue))
  (set `/Game/Enemy/BP_EnemyHitBox.Damage` (`self.Damage`) _returnvalue)
  (`self.K2_AttachToComponent` _output_get (`self.Mesh`) (`self.HitBoxSokectName`) "SnapToTarget" "SnapToTarget" "SnapToTarget" true))

(event `self.ReceiveTick`
  (params (DeltaSeconds :type "Float (single-precision)"))
  (bind (_returnvalue_roll _returnvalue_pitch _returnvalue_yaw) (`KismetMathLibrary.BreakRotator` (`SceneComponent.K2_GetComponentRotation` (`self.CapsuleComponent`))))
  (`SceneComponent.K2_SetRelativeRotation` (`self.Health`) (`KismetMathLibrary.MakeRotator` 0.0 60.0 (`KismetMathLibrary.Abs` (- _returnvalue_yaw 180.0))) false false))

(event `self.CapsuleComponent.OnComponentBeginOverlap`
  (params (OverlappedComponent :type "PrimitiveComponent Object Reference") (OtherActor :type "Actor Object Reference") (OtherComp :type "PrimitiveComponent Object Reference") (OtherBodyIndex :type Integer) (bFromSweep :type Boolean) (SweepResult :type "HitResult Structure (by ref)"))
  (bind _asbp_tssprojectile (cast `/Game/Weapons/BP_TSSProjectile` OtherActor))
  (bind _output_get (set `self.Helath` (- (`self.Helath`) (`/Game/Weapons/BP_TSSProjectile.Damage` _asbp_tssprojectile))))
  (`self.SetHealthText`)
  (if (<= _output_get 0.0)
    (`self.Death`)))

(event `Death`
  (bind (_returnvalue_x _returnvalue_y) (`KismetMathLibrary.BreakVector` (`self.K2_GetActorLocation`)))
  (if (not (`self.IsDead`))
    (`PrimitiveComponent.SetCollisionEnabled` (`self.CapsuleComponent`) "NoCollision")
    (set `self.IsDead` true)
    (`BrainComponent.StopLogic` (`AIController.BrainComponent` (`AIBlueprintHelperLibrary.GetAIController` self)) "")
    (`SceneComponent.SetVisibility` (`self.Health`) false false)
    (bind _asbp_tssbase_game_mode (cast `/Game/BP_TSSBaseGameMode` (`GameplayStatics.GetGameMode`)))
    (set `/Game/BP_TSSBaseGameMode.PlayerScore` (+ (`/Game/BP_TSSBaseGameMode.PlayerScore` _asbp_tssbase_game_mode) (`self.ScorePoints`)) _asbp_tssbase_game_mode)
    (bind _outactors (`GameplayStatics.GetAllActorsOfClass` "/Game/Enemy/EnemiesSpawner/BP_EnemiesSpawner.BP_EnemiesSpawner_C"))
    (`/Game/Enemy/EnemiesSpawner/BPI_EnemiesSwapner.EnemyDeath` (`|GetArrayItem` _outactors))
    (`self.K2_DestroyActor` (`self.HitBoxRef`))
    (if (> (`KismetMathLibrary.RandomIntegerInRange` 0 100) 70)
      (if (>= (`KismetMathLibrary.RandomIntegerInRange` 0 100) 80)
        (set `self.PickupIndex` 1)
        (else
          (set `self.PickupIndex` 0)))
      (`|SpawnActorFromClass` (`|GetArrayItem` (`self.SpawnPickupReferences`) (`self.PickupIndex`)) (`KismetMathLibrary.MakeTransform` (`KismetMathLibrary.MakeVector` _returnvalue_x _returnvalue_y 13.0)) "Undefined" "MultiplyWithRoot" null null))
    (`KismetSystemLibrary.Delay` 1.5)
    (`self.K2_DestroyActor`)))

(fn `SetHealthText`
  (`TextRenderComponent.K2_SetText` (`self.Health`) (`KismetTextLibrary.Conv_DoubleToText` (`self.Helath`) "HalfToEven")))

(fn `UserConstructionScript`)