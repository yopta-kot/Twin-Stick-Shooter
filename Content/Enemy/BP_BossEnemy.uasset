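; BP_BossEnemy is a boss enemy Blueprint that varies its walking speed at random during play.
; After running the parent BeginPlay, it calls ChangeWalkSpeed, which sets the CharacterMovement max walk speed to a random multiple of a base value.
; That event calls itself after a fixed delay, forming an endless re-roll loop without Tick.
; All other behavior is left to the parent class.
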(event `ChangeWalkSpeed`
  (set `CharacterMovementComponent.MaxWalkSpeed` (* (`KismetMathLibrary.RandomFloatInRange` 1.0 2.5) 250.0) (`self.CharacterMovement`))
  (`KismetSystemLibrary.Delay` 5.0)
  (`self.ChangeWalkSpeed`))

(event `self.ReceiveBeginPlay`
  (`parent.ReceiveBeginPlay`)
  (`self.ChangeWalkSpeed`))

(fn `UserConstructionScript`
  (`parent.UserConstructionScript`))