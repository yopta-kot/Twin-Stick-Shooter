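; One-shot trigger actor that spawns a boss enemy once the player has earned enough score.
; When a TSS base character overlaps the Trigger, it checks the game mode's PlayerScore against a fixed threshold of 300.
; On success it spawns BP_BossEnemy offset from the trigger by SpawnLocation, flags it as not auto-spawned, plays a sound and destroys itself.
; Overlaps below the threshold leave the spawner in place.
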(event `self.Trigger.OnComponentBeginOverlap`
  (params (OverlappedComponent :type "PrimitiveComponent Object Reference") (OtherActor :type "Actor Object Reference") (OtherComp :type "PrimitiveComponent Object Reference") (OtherBodyIndex :type Integer) (bFromSweep :type Boolean) (SweepResult :type "HitResult Structure (by ref)"))
  (bind (_spawnlocation_location _spawnlocation_rotation _spawnlocation_scale) (`KismetMathLibrary.BreakTransform` (`self.SpawnLocation`)))
  (bind _returnvalue_location (`KismetMathLibrary.BreakTransform` (`SceneComponent.K2_GetComponentToWorld` (`self.Trigger`))))
  (cast `/Game/Player/BP_TSSBaseCharacter` OtherActor)
  (bind _asbp_tssbase_game_mode (cast `/Game/BP_TSSBaseGameMode` (`GameplayStatics.GetGameMode`)))
  (if (>= (`/Game/BP_TSSBaseGameMode.PlayerScore` _asbp_tssbase_game_mode) 300)
    (bind _returnvalue (`|SpawnActorFromClass` "/Game/Enemy/BP_BossEnemy.BP_BossEnemy_C" (`KismetMathLibrary.MakeTransform` (+ _returnvalue_location _spawnlocation_location) _spawnlocation_rotation _spawnlocation_scale) "Undefined" "MultiplyWithRoot" null null))
    (set `/Game/Enemy/BP_BaseEnemy.IsAutoSpawned?` false _returnvalue)
    (`GameplayStatics.PlaySound2D` "/Game/Enemy/Boss/SFX/SFX_BossSpawned.SFX_BossSpawned" 1.0 1.0 0.0 null null)
    (`self.K2_DestroyActor`)))

(fn `UserConstructionScript`)