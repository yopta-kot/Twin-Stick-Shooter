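; Enemy spawner actor that, while activated, keeps spawning random enemy types at random navigable points around the player up to a population cap.
; Every five seconds it spawns a random-sized batch, shrinking the upper bound near the cap, then re-triggers itself through SpawnEnemy.
; Reaching MaxEnemies halts the loop; EnemyDeath decrements the count and restarts it after a short delay.
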(event `self.ReceiveBeginPlay`
  (bind _enemiesactors (`self.EnemiesActors`))
  (bind _randomarray (`self.RandomArray`))
  (if (`self.IsActivation?`) :!label _label
    (`KismetSystemLibrary.Delay` 5.0)
    ;[1 1 1] Set Max Spawn Enemy
    (switch `int` (- (`self.MaxEnemies`) (`self.EnemiesCount`))
      (:`Default`
        _)
      (:`0`
        (set `self.CanSpawn` false))
      (:`1`
        (set `self.MaxSpawnEnemy` 1))
      (:`2`
        (set `self.MaxSpawnEnemy` 2)))
    (if (`self.CanSpawn`)
      ;[1 1 1] Generate array
      (`KismetArrayLibrary.Array_Resize` _randomarray (`KismetMathLibrary.RandomIntegerInRange` (`self.MinSpawnEnemy`) (`self.MaxSpawnEnemy`)))
      (for _ _randomarray
        (`|SpawnActorFromClass` (`|GetArrayItem` _enemiesactors (`KismetMathLibrary.RandomIntegerInRange` 0 (`KismetArrayLibrary.Array_LastIndex` _enemiesactors))) (`KismetMathLibrary.MakeTransform` (`NavigationSystemV1.K2_GetRandomReachablePointInRadius` (`self.K2_GetActorLocation` (`GameplayStatics.GetPlayerCharacter` 0)) 3000.0 null "/Script/AIModule.NavFilter_AIControllerDefault")) "Undefined" "MultiplyWithRoot" null null)
        (`/Engine/EditorBlueprintResources/StandardMacros.IncrementInt` (`self.EnemiesCount`)))
      (`self.SpawnEnemy`))))

(event `SpawnEnemy`
  (goto _label))

(event `/Game/Enemy/EnemiesSpawner/BPI_EnemiesSwapner.EnemyDeath`
  (`/Engine/EditorBlueprintResources/StandardMacros.DecrementInt` (`self.EnemiesCount`)
    (:`  `
      (if (not (`self.CanSpawn`))
        (`KismetSystemLibrary.Delay` 2.0)
        (set `self.CanSpawn` true)
        (`self.SpawnEnemy`)))))

(fn `UserConstructionScript`)