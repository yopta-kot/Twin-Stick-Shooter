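; BP_EnemySpawner is a trigger-based spawner that creates a random enemy when a BP_TSSBaseCharacter overlaps it.
; It picks a class from EnemiesActors, spawns it at the trigger's location plus SpawnLocation, and clears IsAutoSpawned on BP_BaseEnemy spawns.
; It then disables trigger collision and starts a Delay with nothing wired after it.
; A separate Reactivate event re-enables query collision, but nothing here calls it.
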(event `self.Trigger.OnComponentBeginOverlap`
  (params (OverlappedComponent :type "PrimitiveComponent Object Reference") (OtherActor :type "Actor Object Reference") (OtherComp :type "PrimitiveComponent Object Reference") (OtherBodyIndex :type Integer) (bFromSweep :type Boolean) (SweepResult :type "HitResult Structure (by ref)"))
  (bind _enemiesactors (`self.EnemiesActors`))
  (cast `/Game/Player/BP_TSSBaseCharacter` OtherActor)
  (bind _returnvalue (`|SpawnActorFromClass` (`|GetArrayItem` _enemiesactors (`KismetMathLibrary.RandomIntegerInRange` 0 (`KismetArrayLibrary.Array_LastIndex` _enemiesactors))) (`KismetMathLibrary.MakeTransform` (+ (`SceneComponent.K2_GetComponentLocation` (`self.Trigger`)) (`self.SpawnLocation`))) "Undefined" "MultiplyWithRoot" null null))
  (bind _asbp_base_enemy (cast `/Game/Enemy/BP_BaseEnemy` _returnvalue))
  (set `/Game/Enemy/BP_BaseEnemy.IsAutoSpawned?` false _asbp_base_enemy)
  (`PrimitiveComponent.SetCollisionEnabled` (`self.Trigger`) "NoCollision")
  (`KismetSystemLibrary.Delay` (* 60.0 1.0)))

(event `Reactivate`
  (`PrimitiveComponent.SetCollisionEnabled` (`self.Trigger`) "QueryOnly"))

(fn `UserConstructionScript`)