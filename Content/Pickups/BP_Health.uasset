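; BP_Health is a medkit pickup that heals an overlapping BP_TSSBaseCharacter whose health is below maximum.
; On box overlap it passes current health plus MaxHealing, clamped to MaxHealth, to the character's PickupHealth and plays a 2D pickup sound.
; Static pickups then disable collision, hide the mesh and flag themselves as picked up until the Respawn event restores them, while non-static ones destroy themselves.
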(event `self.Box.OnComponentBeginOverlap`
  (params (OverlappedComponent :type "PrimitiveComponent Object Reference") (OtherActor :type "Actor Object Reference") (OtherComp :type "PrimitiveComponent Object Reference") (OtherBodyIndex :type Integer) (bFromSweep :type Boolean) (SweepResult :type "HitResult Structure (by ref)"))
  (bind _asbp_tssbase_character (cast `/Game/Player/BP_TSSBaseCharacter` OtherActor))
  (bind _health (`/Game/Player/BP_TSSBaseCharacter.Health` _asbp_tssbase_character))
  (bind _maxhealth (`/Game/Player/BP_TSSBaseCharacter.MaxHealth` _asbp_tssbase_character))
  (if (< (- _health _maxhealth) 0.0)
    (`/Game/Player/BP_TSSBaseCharacter.Pickup Health` _asbp_tssbase_character (`KismetMathLibrary.FClamp` (+ _health (`self.MaxHealing`)) 0.0 _maxhealth))
    (`GameplayStatics.PlaySound2D` "/Game/Pickups/SFX/SFX_Medkit_Pickup.SFX_Medkit_Pickup" 1.0 1.0 0.0 null null)
    (if (`self.IsStatic?`)
      (`PrimitiveComponent.SetCollisionEnabled` (`self.Box`) "NoCollision")
      (`SceneComponent.SetVisibility` (`self.Cube`) false true)
      (set `self.IsPickuped?` true)
      (else
        (`self.K2_DestroyActor`)))))

(event `Respawn`
  (`PrimitiveComponent.SetCollisionEnabled` (`self.Box`) "QueryAndPhysics")
  (`SceneComponent.SetVisibility` (`self.Cube`) true true)
  (set `self.IsPickuped?` false))

(fn `UserConstructionScript`)