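; Player character for a top-down shooter, with cursor aiming, walking, pistol fire and door interaction.
; BeginPlay attaches a spawned pistol and adds the HUD, while Tick turns the character toward the cursor hit at constant interpolated speed and counter-rotates the health text.
; Shots consume pistol ammo, and doors respond through BPI_Door.
; Enemy hitbox overlaps reduce health until a one-time ragdoll death reloads the level after a delay.
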(event `self.ReceiveBeginPlay`
  ;[1 1 1] Attach pistol weapon
  (bind _returnvalue (`|SpawnActorFromClass` "/Game/Weapons/BP_TSSPistolWeapon.BP_TSSPistolWeapon_C" (`self.GetTransform`) "Undefined" "MultiplyWithRoot" self self))
  (bind _output_get (set `self.PistolReference` _returnvalue))
  (`self.K2_AttachToComponent` _output_get (`self.Mesh`) "PistolSocket" "SnapToTarget" "SnapToTarget" "SnapToTarget" true)
  ;[1 1 1] Set Health Text
  (`self.SetHealthText`)
  (bind _returnvalue_2 (`|CreateWidget` "/Game/Player/UMG_Default.UMG_Default_C"))
  (`UserWidget.AddToViewport` _returnvalue_2 0))

(event `self.ReceiveTick`
  (params (DeltaSeconds :type "Float (single-precision)"))
  ;[1 1 1] Mouse control
  (bind _newparam (`self.GetRotationByCursor`))
  (`self.K2_SetActorRotation` _newparam)
  ;[1 1 1] Rotate Health Text
  (`SceneComponent.K2_SetRelativeRotation` (`self.HealthText`) (`KismetMathLibrary.MakeRotator` 0.0 60.0 (`KismetMathLibrary.Abs` (- (.yaw _newparam) 180.0))) false false))

(event `EnhancedInput|/Game/Player/Input/Actions/IA_Action`
  (params (ActionValue :type Boolean) (ElapsedSeconds :type "Float (double-precision)") (TriggeredSeconds :type "Float (double-precision)") (InputAction :type "InputAction Object Reference" :default "/Game/Player/Input/Actions/IA_Action.IA_Action"))
  ;[1 1 1] Open/Close door
  (:`Started`
    (for _array_element (`self.GetOverlappingActors` "/Script/Engine.Actor")
      (if (`KismetSystemLibrary.DoesImplementInterface` _array_element "/Game/Blueprints/Door/BPI_Door.BPI_Door_C")
        (message `/Game/Blueprints/Door/BPI_Door.Open/Close Door` _array_element)
        (break)))))

(event `EnhancedInput|/Game/Player/Input/Actions/IA_Walk`
  (params (ActionValue :type "Vector2D Structure") (ElapsedSeconds :type "Float (double-precision)") (TriggeredSeconds :type "Float (double-precision)") (InputAction :type "InputAction Object Reference" :default "/Game/Player/Input/Actions/IA_Walk.IA_Walk"))
  ;[1 1 1] Movement
  (:`Triggered`
    (`self.AddMovementInput` (`KismetMathLibrary.GetRightVector` (struct)) ActionValue_X)
    (`self.AddMovementInput` (`KismetMathLibrary.GetForwardVector` (struct)) ActionValue_Y)))

(event `EnhancedInput|/Game/Player/Input/Actions/IA_Shot`
  (params (ActionValue :type Boolean) (ElapsedSeconds :type "Float (double-precision)") (TriggeredSeconds :type "Float (double-precision)") (InputAction :type "InputAction Object Reference" :default "/Game/Player/Input/Actions/IA_Shot.IA_Shot"))
  (bind _pistolreference (`self.PistolReference`))
  (bind _currentammo (`/Game/Weapons/BP_TSSBaseWeapon.CurrentAmmo` _pistolreference))
  ;[1 1 1] Take a shot
  (:`Started`
    (if (> _currentammo 0)
      (`/Game/Weapons/BP_TSSPistolWeapon.TakeShot` _pistolreference)
      (`/Engine/EditorBlueprintResources/StandardMacros.DecrementInt` _currentammo)
      (else
        (`GameplayStatics.PlaySound2D` "/Game/Weapons/SFX/SFX_Weapon_No_Ammo.SFX_Weapon_No_Ammo" 1.0 1.0 0.0 null null)))))

(event `self.CapsuleComponent.OnComponentBeginOverlap`
  (params (OverlappedComponent :type "PrimitiveComponent Object Reference") (OtherActor :type "Actor Object Reference") (OtherComp :type "PrimitiveComponent Object Reference") (OtherBodyIndex :type Integer) (bFromSweep :type Boolean) (SweepResult :type "HitResult Structure (by ref)"))
  (bind _asbp_enemy_hit_box (cast `/Game/Enemy/BP_EnemyHitBox` OtherActor))
  (bind _output_get (set `self.Health` (- (`self.Health`) (`/Game/Enemy/BP_EnemyHitBox.Damage` _asbp_enemy_hit_box))))
  (`self.SetHealthText`)
  (if (<= _output_get 0.0)
    (`self.Death`)))

(event `Death`
  (bind _mesh (`self.Mesh`))
  (`/Engine/EditorBlueprintResources/StandardMacros.DoOnce` false
    (:`Completed`
      (`SceneComponent.SetVisibility` (`self.HealthText`) false false)
      (set `self.IsDead` true)
      (`CharacterMovementComponent.DisableMovement` (`self.CharacterMovement`))
      (`self.DisableInput` (`GameplayStatics.GetPlayerController` 0))
      (`PrimitiveComponent.SetCollisionEnabled` _mesh "QueryAndPhysics")
      (`PrimitiveComponent.SetCollisionObjectType` _mesh "ECC_PhysicsBody")
      (`PrimitiveComponent.SetSimulatePhysics` _mesh true)
      (`KismetSystemLibrary.Delay` 10.0)
      (bind _returnvalue (`GameplayStatics.GetCurrentLevelName` true))
      (`GameplayStatics.OpenLevel` (`KismetStringLibrary.Conv_StringToName` _returnvalue)))))

(event `Pickup Health`
  (params (NewHealth :type "Float (double-precision)"))
  (set `self.Health` NewHealth)
  (`self.SetHealthText`))

(fn `GetRotationByCursor`
  (returns (NewParam :type "Rotator Structure"))
  (bind (_returnvalue_roll _returnvalue_pitch _returnvalue_yaw) (`KismetMathLibrary.BreakRotator` (`self.K2_GetActorRotation`)))
  (bind (_returnvalue_roll_2 _returnvalue_pitch_2 _returnvalue_yaw_2) (`KismetMathLibrary.BreakRotator` (`KismetMathLibrary.RInterpTo_Constant` (`KismetMathLibrary.MakeRotator` _returnvalue_roll _returnvalue_pitch _returnvalue_yaw) (`KismetMathLibrary.FindLookAtRotation` (`self.StartVector`) (- (`.Location` (`GameplayStatics.BreakHitResult` (`PlayerController.GetHitResultUnderCursorByChannel` (`GameplayStatics.GetPlayerController` 0) "TraceTypeQuery1" true))) (`self.K2_GetActorLocation`))) (`GameplayStatics.GetWorldDeltaSeconds`) 320.0)))
  (return (`KismetMathLibrary.MakeRotator` _returnvalue_roll _returnvalue_pitch _returnvalue_yaw_2)))

(fn `SetHealthText`
  (`TextRenderComponent.K2_SetText` (`self.HealthText`) (`KismetTextLibrary.Conv_DoubleToText` (`self.Health`) "HalfToEven")))

(fn `UserConstructionScript`
  (set `self.Health` (`self.MaxHealth`)))