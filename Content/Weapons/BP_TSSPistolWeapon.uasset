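; Pistol weapon Blueprint that fires projectiles and takes ammo pickups through two functions, with no active event graph logic.
; TakeShot spawns a BP_TSSProjectile at the referenced character's actor transform rather than at a muzzle point, without checking or spending ammo.
; AddAmmo raises CurrentAmmo by a fixed amount with no cap and always returns false.
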(fn `AddAmmo`
  (returns (Check :type Boolean))
  (set `self.CurrentAmmo` (+ (`self.CurrentAmmo`) 10))
  (return false))

(fn `TakeShot`
  (`|SpawnActorFromClass` "/Game/Weapons/BP_TSSProjectile.BP_TSSProjectile_C" (`self.GetTransform` (`self.CharacterReference`)) "Undefined" "MultiplyWithRoot" null null))

(fn `UserConstructionScript`
  (`parent.UserConstructionScript`))